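; Player controller for team-based gameplay in which the player selects grid cells and builds towers or barracks on them.
; It stores team, color and game mode, creates the gameplay UI and hides the loading screen through the game instance.
; Left click traces under the cursor, highlights only the hit GridBase and enables building.
; Building deducts coins from the player state and has the selected grid spawn the structure.
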(event Custom|SetColorEnumAndTeamMult
  (params (Team :type Integer) (ColorEnum :type Integer))
  ;[1 1 1] ControllerIncludedInTheTeamWithColor
  (Variables|Default|SetTeam Team)
  (Variables|Default|SetColorEnum ColorEnum))

(event Custom|SetGameMode
  (params (GameMode :type Integer))
  ;[1 1 1] SetUpPlayerForNewGameMode
  (Variables|Default|SetGameMode GameMode))

(event Custom|BuildTowerOrBarracs
  (params (NumberOfBuilds :type Integer))
  (bind _playerstate (Variables|GetPlayerState))
  (bind _asmy_player_state (Utilities|Casting|CastToMyPlayerState _playerstate))
  ;[1 1 1] Building
  (if (Variables|Default|GetCanBuild)
    (if (>= (Variables|/Game/Blueprints/Gameplay/MyPlayerState.MyPlayerState_C|GetCoins _asmy_player_state) 5)
      (Variables|/Game/Blueprints/Gameplay/MyPlayerState.MyPlayerState_C|SetCoins _asmy_player_state (- (Variables|/Game/Blueprints/Gameplay/MyPlayerState.MyPlayerState_C|GetCoins _asmy_player_state) 5))
      (Variables|Default|SetNumberOfBuilds NumberOfBuilds)
      (Variables|Default|SetCanBuild false)
      (Default|SpawnBuilds (Variables|Default|GetSelectedGrid) (Variables|Default|GetNumberOfBuilds) (Variables|Default|GetLocationBuild)))))

(event Custom|SetColorEnumAndTeam
  (params (Team :type Integer) (ColorEnum :type Integer))
  ;[1 1 1] ControllerIncludedInTheTeamWithColor
  (Variables|Default|SetTeam Team)
  (Variables|Default|SetColorEnum ColorEnum))

(event Custom|UpdateAllVariables
  (params (SelectedGrid :type Grid%20Base%20Object%20Reference) (NumberOfBuilds :type Integer) (LocationBuild :type Vector) (Team :type Integer) (ColorEnum :type Integer))
  (Variables|Default|SetCanBuild true)
  (Variables|Default|SetSelectedGrid SelectedGrid)
  (Variables|Default|SetNumberOfBuilds NumberOfBuilds)
  (Variables|Default|SetLocationBuild LocationBuild)
  (Variables|Default|SetTeam Team)
  (Variables|Default|SetColorEnum ColorEnum))

(event Custom|HideLoadingScreen
  ;[1 1 1] SetUpPlayerForNewGameMode
  (bind _asmy_game_instance (Utilities|Casting|CastToMyGameInstance (Game|GetGameInstance)))
  (Default|HideLoadingScreen _asmy_game_instance))

(event Custom|CreateGameUI
  ;[1 1 1] SetUpPlayerForNewGameMode
  (bind _returnvalue (UserInterface|CreateWidget "/Game/UI/GameplayUI/GameplayWB.GameplayWB_C"))
  (bind _output_get (Variables|Default|SetGamePlayWB _returnvalue))
  (UserInterface|Viewport|AddtoViewport _output_get 0)
  (Input|SetInputModeGameandUI self (Variables|Default|GetGamePlayWB) "DoNotLock" false)
  (Variables|Default|SetbShowMouseCursor true))

(event EventBeginPlay
  ;[1 1 1] SetUpPlayerForNewGameMode
  (Variables|Default|SetbShowMouseCursor true))

(event Input|MouseEvents|LeftMouseButton
  (params (Key :type Key%20Structure))
  (bind _returnvalue (Game|GetPlayerController 0))
  (bind (_worldlocation _worlddirection) (Game|Player|ConvertMouseLocationToWorldSpace _returnvalue))
  (:Pressed
    (bind (_outhit _returnvalue_2) (Collision|LineTraceForObjects _worldlocation (+ _worldlocation (* _worlddirection 2e+03)) (Utilities|Array|MakeArray "ObjectTypeQuery7") false (Utilities|Array|MakeArray self) "None"))
    (if _returnvalue_2
      (bind _outactors (Actor|GetAllActorsOfClass "/Game/Blueprints/Gameplay/Grid/GridBase.GridBase_C"))
      (for _array_element _outactors
        (Rendering|SetVisibility (Variables|/Game/Blueprints/Gameplay/Grid/GridBase.GridBase_C|GetPlane _array_element) false false))
      (bind _asgrid_base (Utilities|Casting|CastToGridBase (.HitActor (Collision|BreakHitResult _outhit))))
      (bind _output_get (Variables|Default|SetSelectedGrid _asgrid_base))
      (Variables|Default|SetLocationBuild (Variables|/Game/Blueprints/Gameplay/Grid/GridBase.GridBase_C|GetLocationGrid _output_get))
      (CallFunction|UpdateAllVariables (Variables|Default|GetSelectedGrid) (Variables|Default|GetNumberOfBuilds) (Variables|Default|GetLocationBuild) (Variables|Default|GetTeam) (Variables|Default|GetColorEnum))
      (Rendering|SetVisibility (Variables|/Game/Blueprints/Gameplay/Grid/GridBase.GridBase_C|GetPlane _output_get) true false))))

(event Input|KeyboardEvents|Tab
  (params (Key :type Key%20Structure))
  (:Pressed
    (bind _returnvalue (UserInterface|CreateWidget "/Game/UI/GameplayUI/GameplayWB.GameplayWB_C"))
    (UserInterface|Viewport|AddtoViewport _returnvalue 0)))

(fn ConstructionScript)