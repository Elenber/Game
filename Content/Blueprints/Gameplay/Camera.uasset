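; Camera pawn that the player moves around the world with the MoveForward and MoveRight axes.
; Each axis feeds AddMovementInput along world X or Y, so movement ignores the camera's facing.
; An unconnected, never-run chain line-traces forward from the camera to show the hit GridBase's Plane and hide all others.
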(event Input|AxisEvents|InputAxisMoveForward
  (params (AxisValue :type Float%20%28single-precision%29))
  (Pawn|Input|AddMovementInput (Math|Vector|MakeVector AxisValue 0.0 0.0) 1.0 false))

(event Input|AxisEvents|InputAxisMoveRight
  (params (AxisValue :type Float%20%28single-precision%29))
  (Pawn|Input|AddMovementInput (Math|Vector|MakeVector 0.0 AxisValue 0.0) 1.0 false))

(event Input|MouseEvents|LeftMouseButton
  (params (Key :type Key%20Structure))
  ;[1 1 1] Пока Оставлю 13.07.18
)

(fn ConstructionScript)