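; PawnCamera is a player pawn that moves on world X and Y from input axes and spawns buildings for its team.
; It receives a material instance and team from the player controller, storing them and forwarding them through a second "Mult" event.
; SpawnBuilds relays location and index to SpawnBuildsOwning, which spawns the selected Builds class with the pawn as owner, rotated to opposite sides depending on team.
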(event Custom|SpawnBuilds
  (params (BuildLocation :type Vector) (NumberOfBuilds :type Integer))
  ;[1 1 1] Building
  (bind _output_get (Variables|Building|SetBuildLocation BuildLocation))
  (bind _output_get_2 (Variables|Building|SetNumberOfBuilds NumberOfBuilds))
  (CallFunction|SpawnBuildsOwning _output_get _output_get_2))

(event Custom|GetFromPCVar
  (params (MaterialInstance :type Material%20Instance%20Object%20Reference) (Team :type Integer))
  ;[1 1 1] GetVariablesFromPlayerController
  (bind _output_get (Variables|Building|SetMaterialInstance MaterialInstance))
  (bind _output_get_2 (Variables|Default|SetTeam Team))
  (CallFunction|GetfromPCVarMult _output_get _output_get_2))

(event Custom|GetFromPCVarMult
  (params (MaterialInstance :type Material%20Instance%20Object%20Reference) (Team :type Integer))
  ;[1 1 1] GetVariablesFromPlayerController
  (Variables|Building|SetMaterialInstance MaterialInstance)
  (Variables|Default|SetTeam Team))

(event Custom|SpawnBuildsOwning
  (params (Spawn%20Transform%20Location :type Vector) (NumberOfBuilds :type Integer))
  ;[1 1 1] Building
  (Variables|Building|SetNumberOfBuilds NumberOfBuilds)
  (if (== (Variables|Default|GetTeam) 1)
    (Variables|Default|SetRotateBuild "0,-90.000000, 0")
    (else
      (Variables|Default|SetRotateBuild "0,90.000000, 0")))
  (Game|SpawnActorfromClass (Utilities|Array|Get(acopy) (Variables|Building|GetBuilds) (Variables|Building|GetNumberOfBuilds)) (Math|Transform|MakeTransform Spawn%20Transform%20Location (Variables|Default|GetRotateBuild) "1,1,1") "Undefined" self (Game|GetInstigator)))

(event Input|AxisEvents|InputAxisMoveForward
  (params (AxisValue :type Float%20%28single-precision%29))
  ;[1 1 1] Movement
  (Pawn|Input|AddMovementInput (Math|Vector|MakeVector AxisValue 0.0 0.0) 1.0 false))

(event Input|AxisEvents|InputAxisMoveRight
  (params (AxisValue :type Float%20%28single-precision%29))
  ;[1 1 1] Movement
  (Pawn|Input|AddMovementInput (Math|Vector|MakeVector 0.0 AxisValue 0.0) 1.0 false))

(fn ConstructionScript)