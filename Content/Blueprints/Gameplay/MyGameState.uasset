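; Game state that tracks which player colors are still available and shares that list with every player state.
; SwitchOffColorEnum overwrites the chosen color's entry in AvailableColors and copies the array to each MyPlayerState in PlayerArray.
; Inside that loop it also calls SwitchOffColorEnumMult, which repeats the same update and copy.
; The OnRep handler for AvailableColors is empty.
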(event Custom|SwitchOffColorEnum
  (params (ColorEnum :type Integer))
  (bind _output_get (Variables|Default|SetColorEnum ColorEnum))
  (Utilities|Array|SetArrayElem (Variables|Default|GetAvailableColors) _output_get false)
  (for _array_element (Variables|Default|GetPlayerArray)
    (bind _asmy_player_state (Utilities|Casting|CastToMyPlayerState _array_element))
    (Variables|/Game/Blueprints/Gameplay/MyPlayerState.MyPlayerState_C|SetAvailableColors _asmy_player_state (Variables|Default|GetAvailableColors))
    (CallFunction|SwitchOffColorEnumMult (Variables|Default|GetColorEnum))))

(event Custom|SwitchOffColorEnumMult
  (params (ColorEnum :type Integer))
  (bind _output_get (Variables|Default|SetColorEnum ColorEnum))
  (Utilities|Array|SetArrayElem (Variables|Default|GetAvailableColors) _output_get false)
  (for _array_element (Variables|Default|GetPlayerArray)
    (bind _asmy_player_state (Utilities|Casting|CastToMyPlayerState _array_element))
    (Variables|/Game/Blueprints/Gameplay/MyPlayerState.MyPlayerState_C|SetAvailableColors _asmy_player_state (Variables|Default|GetAvailableColors))))

(event EventBeginPlay)

(fn ConstructionScript)

(fn OnRepAvailableColors)